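; Player gun component for a target-shooting minigame that shows the character's gun with ammo and crosshair widgets.
; Shooting line-traces from the first-person camera and spends ammo, while a timed reload refills it to a capacity set by the ammo upgrade flag.
; Hit targets optionally spin, spawn a Niagara effect, add or subtract points and are destroyed.
; Clearing the last target finishes the minigame.
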(event `self.ReceiveBeginPlay`
  (bind _asbp_first_person_character_master (cast `/Game/_Developer/Sam/Blueprints/BP_FirstPersonCharacter_Master` (`GameplayStatics.GetPlayerCharacter` 0)))
  (bind _output_get (set `self.FirstPersonCharacter` _asbp_first_person_character_master))
  (`SceneComponent.SetVisibility` (`/Game/_Developer/Sam/Blueprints/BP_FirstPersonCharacter_Master.Gun` _output_get) true true)
  (bind _returnvalue (`|CreateWidget` "/Game/Developer/BenH/UI/AmmoUpgrade/WBP_Ammo.WBP_Ammo_C"))
  (bind _output_get_2 (set `self.CurrentAmmoWidget` _returnvalue))
  (set `/Game/Developer/BenH/UI/AmmoUpgrade/WBP_Ammo.CurrentAmmo` (`KismetTextLibrary.Conv_IntToText` (`self.Ammo`)) (`self.CurrentAmmoWidget`))
  (`UserWidget.AddToViewport` _output_get_2 0)
  (bind _returnvalue_2 (`|CreateWidget` "/Game/Developer/BenH/UI/Crosshair/WBP_Crosshair.WBP_Crosshair_C"))
  (`UserWidget.AddToViewport` _returnvalue_2 0)
  (if (`self.bAmmoUpgrade`)
    (set `self.Ammo` 8)
    (set `/Game/Developer/BenH/UI/AmmoUpgrade/WBP_Ammo.MaxAmmo` "8" (`self.CurrentAmmoWidget`))
    (set `self.bHasAmmo` true)
    (else
      (set `self.Ammo` 6)
      (set `/Game/Developer/BenH/UI/AmmoUpgrade/WBP_Ammo.MaxAmmo` "6" (`self.CurrentAmmoWidget`))
      (set `self.bHasAmmo` true))))

(event `EnhancedInput|/Game/Developer/BenH/Actions/IA_Reload`
  (params (ActionValue :type Boolean) (ElapsedSeconds :type "Float (double-precision)") (TriggeredSeconds :type "Float (double-precision)") (InputAction :type "InputAction Object Reference" :default "/Game/Developer/BenH/Actions/IA_Reload.IA_Reload"))
  ;[0.15 0.15 0.5395 0.502] Reload
  (:`Started`
    (`KismetSystemLibrary.PrintString` "Reloading..." true true (struct :`G` 0.66 :`B` 1.0 :`A` 1.0) 3.0)
    (`KismetSystemLibrary.Delay` (`self.Reload Time`))
    (if (`self.AmmoUpgrade`)
      (set `self.Ammo` 8)
      (set `/Game/Developer/BenH/UI/AmmoUpgrade/WBP_Ammo.CurrentAmmo` (`KismetTextLibrary.Conv_IntToText` (`self.Ammo`)) (`self.CurrentAmmoWidget`))
      (set `/Game/Developer/BenH/UI/AmmoUpgrade/WBP_Ammo.MaxAmmo` "8" (`self.CurrentAmmoWidget`))
      (set `self.Has Ammo` true)
      (`KismetSystemLibrary.PrintString` "Fully Reloaded! Fire Away!")
      (else
        (set `self.Ammo` 6)
        (set `/Game/Developer/BenH/UI/AmmoUpgrade/WBP_Ammo.CurrentAmmo` (`KismetTextLibrary.Conv_IntToText` (`self.Ammo`)) (`self.CurrentAmmoWidget`))
        (set `/Game/Developer/BenH/UI/AmmoUpgrade/WBP_Ammo.MaxAmmo` "6" (`self.CurrentAmmoWidget`))
        (set `self.Has Ammo` true)
        (`KismetSystemLibrary.PrintString` "Fully Reloaded! Fire Away!")))))

(event `EnhancedInput|/Game/Developer/BenH/Actions/IA_Shoot`
  (params (ActionValue :type Boolean) (ElapsedSeconds :type "Float (double-precision)") (TriggeredSeconds :type "Float (double-precision)") (InputAction :type "InputAction Object Reference" :default "/Game/Developer/BenH/Actions/IA_Shoot.IA_Shoot"))
  (bind _firstpersoncamera (`/Game/_Developer/Sam/Blueprints/BP_FirstPersonCharacter_Master.FirstPersonCamera` (`self.FirstPersonCharacter`)))
  (bind _returnvalue (`SceneComponent.K2_GetComponentLocation` _firstpersoncamera))
  ;[0.15 0.15 0.542 0.5] Fire
  (:`Started`
    (if (`self.Has Ammo`)
      (`KismetSystemLibrary.PrintString` "Pow!")
      (bind _outhit (`KismetSystemLibrary.LineTraceSingle` :`Start` _returnvalue :`End` (+ _returnvalue (* (`SceneComponent.GetForwardVector` _firstpersoncamera) (`self.RayDistance`))) :`TraceChannel` "TraceTypeQuery1" :`DrawDebugType` "ForDuration"))
      (`|ExecutionSequence`
        (:`then_0`
          (bind (_bblockinghit _binitialoverlap _time _distance _location _impactpoint _normal _impactnormal _physmat _hitactor) (`GameplayStatics.BreakHitResult` _outhit))
          (`KismetSystemLibrary.PrintString` (`KismetStringLibrary.Conv_ObjectToString` _hitactor))
          (`KismetSystemLibrary.PrintString` "FEEWWW!")
          (set `self.Ammo` (- (`self.Ammo`) 1))
          (set `/Game/Developer/BenH/UI/AmmoUpgrade/WBP_Ammo.CurrentAmmo` (`KismetTextLibrary.Conv_IntToText` (`self.Ammo`)) (`self.CurrentAmmoWidget`))
          (`KismetSystemLibrary.PrintString` (`KismetStringLibrary.Concat_StrStr` "You have " (`KismetStringLibrary.Conv_IntToString` (`self.Ammo`)) " bullets left"))
          (if (<= (`self.Ammo`) 0)
            (set `self.Has Ammo` false)))
        (:`then_1`
          (bind _asbp_master_target (cast `/Game/Developer/BenH/Blueprints/BP_MasterTarget` _hitactor))
          (if (`/Game/Developer/BenH/Blueprints/BP_MasterTarget.DoesSpin?` _asbp_master_target)
            (`/Game/Developer/BenH/Blueprints/BP_MasterTarget.Rotate` _asbp_master_target)
            (`KismetSystemLibrary.Delay` 1.0))
          (`NiagaraFunctionLibrary.SpawnSystemAtLocation` "/Game/Developer/BenH/Niagara/NS_ChinaBowl.NS_ChinaBowl" (`SceneComponent.K2_GetComponentLocation` (`/Game/Developer/BenH/Blueprints/BP_MasterTarget.TargetMesh` _asbp_master_target)))
          (if (`/Game/Developer/BenH/Blueprints/BP_MasterTarget.LosingPointTarget?` _asbp_master_target)
            (bind _getpoints (`/Game/Developer/BenH/Blueprints/Interfaces/BPI_Points.GetPoints` _asbp_master_target))
            (set `self.Points` (- (`self.Points`) _getpoints))
            (`Actor.K2_DestroyActor` _asbp_master_target)
            (else
              (bind _getpoints_2 (message `/Game/Developer/BenH/Blueprints/Interfaces/BPI_Points.GetPoints` _asbp_master_target))
              (set `self.Points` (+ _getpoints_2 (`self.Points`)))
              (`Actor.K2_DestroyActor` _asbp_master_target)))
          (bind _outactors (`GameplayStatics.GetAllActorsOfClass` "/Game/Developer/BenH/Blueprints/BP_MasterTarget.BP_MasterTarget_C"))
          (if (`KismetArrayLibrary.Array_IsEmpty` _outactors)
            (`self.FinishMingame`))))
      (else
        (`KismetSystemLibrary.PrintString` "You're out of ammo! Press R to Reload!")))))

(fn `CalculatePoints`
  (params (Time :type Integer))
  (returns (Points :type Integer))
  (return 0))

(fn `GetPoints`
  (returns (GetPoints :type Integer))
  (return 0))