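; BP_ChinaDropOffPoint is a drop-off actor that scores and clears china carried by BP_FirstPersonCharacter_Master_BenCopy.
; On overlap, it resets that character's ChinaItemCount, adds a fixed Points reward and calls ChinaSpeed, even without HasChina set.
; If HasChina is set, it also clears the flag and destroys a BP_ChinaBowl found by GetActorOfClass, rather than a tracked carried instance.
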(event `self.ReceiveActorBeginOverlap`
  (params (OtherActor :type "Actor Object Reference"))
  (`|ExecutionSequence`
    (:`then_0`
      (bind _asbp_first_person_character_master_ben_copy (cast `/Game/Developer/BenH/Characters/BP_FirstPersonCharacter_Master_BenCopy` OtherActor))
      (set `/Game/Developer/BenH/Characters/BP_FirstPersonCharacter_Master_BenCopy.ChinaItemCount` 0 _asbp_first_person_character_master_ben_copy)
      (set `/Game/Developer/BenH/Characters/BP_FirstPersonCharacter_Master_BenCopy.Points` (+ (`/Game/Developer/BenH/Characters/BP_FirstPersonCharacter_Master_BenCopy.Points` _asbp_first_person_character_master_ben_copy) 250) _asbp_first_person_character_master_ben_copy)
      (`/Game/Developer/BenH/Characters/BP_FirstPersonCharacter_Master_BenCopy.ChinaSpeed` _asbp_first_person_character_master_ben_copy))
    (:`then_1`
      (bind _asbp_first_person_character_master_ben_copy_2 (cast `/Game/Developer/BenH/Characters/BP_FirstPersonCharacter_Master_BenCopy` OtherActor))
      (if (`/Game/Developer/BenH/Characters/BP_FirstPersonCharacter_Master_BenCopy.HasChina?` _asbp_first_person_character_master_ben_copy_2)
        (bind _asbp_china_bowl (castclass `/Game/Developer/BenH/Blueprints/BP_ChinaBowl` "/Game/Developer/BenH/Blueprints/BP_ChinaBowl.BP_ChinaBowl_C"))
        (bind _returnvalue (`GameplayStatics.GetActorOfClass` _asbp_china_bowl))
        (`self.K2_DestroyActor` _returnvalue)
        (set `/Game/Developer/BenH/Characters/BP_FirstPersonCharacter_Master_BenCopy.HasChina?` false _asbp_first_person_character_master_ben_copy_2)))))

(fn `UserConstructionScript`)