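; Configurable scoring target that displays its point value and can optionally move along a spline.
; The construction script applies an outline overlay, then takes mesh and points from custom overrides or the selected DTABLE_Targets row.
; When Movable, Tick advances the target along TargetPathSpline at a set speed, resetting to the start if Loop is set.
; Rotate activates the RotatingMovement component, and GetPoints returns the score truncated to an integer.
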(event `self.ReceiveBeginPlay`)

(event `self.ReceiveTick`
  (params (DeltaSeconds :type "Float (single-precision)"))
  (if (`self.Movable`)
    (bind _output_get (set `self.Position_On_Spline` (+ (* DeltaSeconds (`self.Speed_On_Spline`)) (`self.Position_On_Spline`))))
    (`SceneComponent.K2_SetWorldTransform` (`self.Target`) (`SplineComponent.GetTransformAtDistanceAlongSpline` (`self.TargetPathSpline`) _output_get "World" false) false false)
    (if (`self.Loop`)
      (if (>= (`self.Position_On_Spline`) (`SplineComponent.GetSplineLength` (`self.TargetPathSpline`)))
        (set `self.Position_On_Spline` 0.0)))))

(event `Rotate`
  (`ActorComponent.Activate` (`self.RotatingMovement`) false))

(fn `GetPoints`
  (returns (GetPoints :type Integer))
  (return (`KismetMathLibrary.FTrunc` (`self.Points`))))

(fn `UserConstructionScript`
  (`MeshComponent.SetOverlayMaterial` (`self.TargetMesh`) (`self.OutlineColor`) false 0)
  (if (`self.Custom?`)
    (`StaticMeshComponent.SetStaticMesh` (`self.TargetMesh`) (`self.CustomMesh`))
    (bind _output_get (set `self.Points` (`self.CustomPoints`)))
    (`TextRenderComponent.K2_SetText` (`self.Score`) (`KismetTextLibrary.Conv_DoubleToText` _output_get "HalfToEven"))
    (else
      (bind _returnvalue (`|GetDataTableRow` "/Game/Developer/BenH/DataTables/DTABLE_Targets.DTABLE_Targets" (`.RowName` (break `DataTableRowHandle` (`self.Selection`))))
        (:`then`
          (bind (_mesh _points) (break `/Game/Developer/BenH/DataTables/STRUCT_Targets` _returnvalue))
          (`StaticMeshComponent.SetStaticMesh` (`self.TargetMesh`) _mesh)
          (set `self.Points` _points)
          (`TextRenderComponent.K2_SetText` (`self.Score`) (`KismetTextLibrary.Conv_DoubleToText` _points "HalfToEven")))))))